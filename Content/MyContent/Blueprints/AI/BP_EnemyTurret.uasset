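; BP_EnemyTurret is an AI turret that turns toward the player and shoots projectiles at them.
; When PawnSensing sees a DroidFirstPersonCharacter, the whole actor snaps to a look-at rotation toward it.
; It then spawns a FirstPersonProjectile at ProjectileSpawnLocation and launches it with an impulse along the Cylinder's forward vector.
; A SpawnProjectile flag with a short Delay limits the fire rate.
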(event `self.PawnSensing.OnSeePawn`
  (params (Pawn :type "Pawn Object Reference"))
  (bind _asdroid_first_person_character (cast `/Game/MyContent/Blueprints/DroidFirstPersonCharacter` Pawn))
  (`|ExecutionSequence`
    (:`then_0`
      ;[1 1 1] Rotate Turret to face target
      (`self.K2_SetActorRotation` (`KismetMathLibrary.FindLookAtRotation` (`self.K2_GetActorLocation`) (`self.K2_GetActorLocation` _asdroid_first_person_character))))
    (:`then_1`
      ;[1 1 1] Shoot projectile at target
      (if (`self.SpawnProjectile`)
        (bind _returnvalue (`|SpawnActorFromClass` "/Game/MyContent/Blueprints/FirstPersonProjectile.FirstPersonProjectile_C" (`SceneComponent.K2_GetComponentToWorld` (`self.ProjectileSpawnLocation`)) "Undefined" "OverrideRootScale" null null))
        (`PrimitiveComponent.AddImpulse` (`/Game/MyContent/Blueprints/FirstPersonProjectile.Sphere` _returnvalue) (* (`SceneComponent.GetForwardVector` (`self.Cylinder`)) (`self.ShootForce`)) "None" true)
        (set `self.SpawnProjectile` false)
        (`KismetSystemLibrary.Delay` 1.5)
        (set `self.SpawnProjectile` true)))))

(fn `UserConstructionScript`)